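; BP_Boat is a boat actor that adjusts to a BP_Water surface and carries an aimable gun.
; On begin play it finds the water, calculates its width and length from four corner points, and caches their world locations.
; Each tick it derives rotation from those cached points and updates its height.
; Events swap head and gun materials for hover feedback and turn the gun toward a target point with a timeline lerp.
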(event EventBeginPlay
  (bind _boatpoints (Variables|Default|GetBoatPoints))
  (bind _returnvalue (Actor|GetActorOfClass "/Game/BP_Water.BP_Water_C"))
  (Variables|Default|SetWater _returnvalue)
  (Class|Boat|CalculateBoatWidthLength (Variables|/Script/Engine.SceneComponent|GetRelativeLocation (Variables|Default|Getx1)) (Variables|/Script/Engine.SceneComponent|GetRelativeLocation (Variables|Default|Getx2)) (Variables|/Script/Engine.SceneComponent|GetRelativeLocation (Variables|Default|Getx3)) (Variables|/Script/Engine.SceneComponent|GetRelativeLocation (Variables|Default|Getx4)))
  (Utilities|Array|Add _boatpoints (Transformation|GetWorldLocation (Variables|Default|Getx1)))
  (Utilities|Array|Add _boatpoints (Transformation|GetWorldLocation (Variables|Default|Getx2)))
  (Utilities|Array|Add _boatpoints (Transformation|GetWorldLocation (Variables|Default|Getx3)))
  (Utilities|Array|Add _boatpoints (Transformation|GetWorldLocation (Variables|Default|Getx4))))

(event Collision|EventActorBeginOverlap
  (params (OtherActor :type Actor%20Object%20Reference)))

(event EventTick
  (params (DeltaSeconds :type Float%20%28single-precision%29))
  (bind _returnvalue (Class|Boat|GetNewBoatRotation (Variables|Default|GetBoatPoints)))
  (Transformation|SetRelativeRotation (Variables|Default|GetBoat) _returnvalue false false)
  (Class|Boat|SetNewBoatHeight))

(event EventChangeHeadandGunMaterial
  (params (isHovered :type Boolean))
  (if isHovered
    (Rendering|Material|SetMaterial (Variables|Default|GetHead) 0 "/Game/Materials/MI_JustColorHovered.MI_JustColorHovered")
    (Rendering|Material|SetMaterial (Variables|Default|GetGun) 0 "/Game/Materials/MI_JustColorHovered.MI_JustColorHovered")
    (else
      (Rendering|Material|SetMaterial (Variables|Default|GetHead) 0 "/Game/Materials/MI_JustColorUnhovered.MI_JustColorUnhovered")
      (Rendering|Material|SetMaterial (Variables|Default|GetGun) 0 "/Game/Materials/MI_JustColorUnhovered.MI_JustColorUnhovered"))))

(event EventAimtoPoint
  (params (point :type Vector :default "0, 0, 0"))
  (bind _gun (Variables|Default|GetGun))
  (bind _alpha (Timeline|Rotate PlayFromStart)
    (:Update
      (Transformation|SetWorldRotation (Variables|Default|GetGun) (Math|Rotator|Lerp(Rotator) (Transformation|GetWorldRotation _gun) (Math|Rotator|FindLookatRotation (Transformation|GetWorldLocation _gun) point) _alpha true) false false))))

(fn ConstructionScript)